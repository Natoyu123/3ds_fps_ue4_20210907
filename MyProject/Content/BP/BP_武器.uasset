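; Weapon Blueprint (BP_武器) that handles automatic fire, magazine reloading and ammo resupply.
; Holding the 開槍 input runs a Delay-paced loop that spawns BP_子彈 at the muzzle socket, passes it weapon damage, plays a muzzle flash and decrements the magazine.
; Custom event 換彈匣 refills the magazine from reserve ammo, taking whatever remains if short.
; Custom event 補充子彈 adds one magazine's worth to the reserve, clamped to its maximum.
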(event Custom|換彈匣
  ;[1 1 1] 計算補充子彈的數量
  (Variables|Default|Set要補充的子彈數量 (- (Variables|Default|Get彈匣容量) (Variables|Default|Get目前子彈數量)))
  ;[1 1 1] 判斷總數是否>=要補充的數量
  (if (>= (Variables|Default|Get子彈總數) (Variables|Default|Get要補充的子彈數量))
    _
    (else
      ;[1 1 1] 總數<要補充的量:把剩餘的都填充
      (Variables|Default|Set要補充的子彈數量 (Variables|Default|Get子彈總數))))
  ;[1 1 1] 目前子彈以及總數更新
  (Variables|Default|Set目前子彈數量 (+ (Variables|Default|Get目前子彈數量) (Variables|Default|Get要補充的子彈數量)))
  (Variables|Default|Set子彈總數 (- (Variables|Default|Get子彈總數) (Variables|Default|Get要補充的子彈數量))))

(event Custom|補充子彈
  ;[1 1 1] 拿取子彈箱並補充子彈
  (bind _output_get (Variables|Default|Set子彈總數 (+ (Variables|Default|Get子彈總數) (Variables|Default|Get彈匣容量))))
  (Variables|Default|Set子彈總數 (Math|Integer|Clamp(Integer) _output_get 0 (Variables|Default|Get子彈上限))))

(event Input|ActionEvents|InputAction開槍
  (params (Key :type Key%20Structure :default "None"))
  (bind _武器模型 (Variables|Default|Get武器模型))
  ;[1 1 1] 開槍
  (:Pressed
    (Variables|Default|Set開槍中 true)
    (if (and (> (Variables|Default|Get目前子彈數量) 0) (Variables|Default|Get開槍中)) :!label _label
      (bind _returnvalue (Game|SpawnActorfromClass "/Game/BP/BP_子彈.BP_子彈_C" (Transformation|GetSocketTransform (Variables|Default|Get武器模型) "子彈插槽" "RTS_World") "Undefined" 0 0)) ; 生成子彈藍圖
      (Variables|/Game/BP/BP_子彈.BP_子彈_C|Set目前武器傷害 _returnvalue (Variables|Default|Get武器傷害))
      (Effects|SpawnEmitteratLocation "/Game/InfinityBladeEffects/Effects/FX_Monsters/FX_Monster_Gruntling/Master/P_BackPack_MuzzleFlash.P_BackPack_MuzzleFlash" (Transformation|GetSocketLocation _武器模型 "子彈插槽") (Transformation|GetSocketRotation _武器模型 "None") "0.100000,0.100000,0.100000") ; 生成粒子在指定座標上
      (Variables|Default|Set目前子彈數量 (- (Variables|Default|Get目前子彈數量) 1))
      (Utilities|FlowControl|Delay (Variables|Default|Get開槍間隔))
      (goto _label)))
  (:Released
    (Variables|Default|Set開槍中 false)))

(fn ConstructionScript)